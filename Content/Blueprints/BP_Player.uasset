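; Player Blueprint with Enhanced Input walking and a timed dash aimed with the mouse cursor.
; BeginPlay adds the input mapping and shows the cursor.
; Dash takes its direction from player and mouse screen positions, then Tick overrides movement velocity while dashing.
; A CanHit flag is set during the dash; capsule hits end the dash and clear the flag after a brief delay.
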(event `self.ReceiveBeginPlay`
  (`|ExecutionSequence`
    (:`then_0`
      ;[1 1 1] Set Player Controller
      (set `self.PlayerController` (`GameplayStatics.GetPlayerController` 0)))
    (:`then_1`
      ;[1 1 1] Enable Player Mapping
      (bind _asplayer_controller (cast `PlayerController` (`self.PlayerController`)))
      (`EnhancedInputSubsystemInterface.AddMappingContext` (pcsubsystem `EnhancedInputLocalPlayerSubsystem` _asplayer_controller) "/Game/Input/PlayerMapping.PlayerMapping" 0 (struct)))
    (:`then_2`
      ;[1 1 1] Show Mouse
      (set `PlayerController.bShowMouseCursor` true (`self.PlayerController`)))))

(event `self.ReceiveTick`
  (params (DeltaSeconds :type "Float (single-precision)"))
  (`|ExecutionSequence`
    (:`then_0`
      ;[0.3765 0.6863 1] Add dash force if dashing
      (if (`self.dashing`)
        (set `MovementComponent.Velocity` (* (`self.dashDirection`) 100 (`self.dashSpeed`)) (`self.CharacterMovement`))))))

(event `EnhancedInput|/Game/Input/Walk`
  (params (ActionValue :type "Vector2D Structure") (ElapsedSeconds :type "Float (double-precision)") (TriggeredSeconds :type "Float (double-precision)") (InputAction :type "InputAction Object Reference" :default "/Game/Input/Walk.Walk"))
  ;[1 0.1569 0.1961] Get Walk Input
  (:`Triggered`
    ;[0.3765 0.6863 1] Walk
    (`self.AddMovementInput` (`KismetMathLibrary.Conv_Vector2DToVector` ActionValue))))

(event `EnhancedInput|/Game/Input/Dash`
  (params (ActionValue :type Boolean) (ElapsedSeconds :type "Float (double-precision)") (TriggeredSeconds :type "Float (double-precision)") (InputAction :type "InputAction Object Reference" :default "/Game/Input/Dash.Dash"))
  ;[1 0.1569 0.1961] Get Dash Input
  (:`Triggered`
    (bind _dashdirection (`self.GetDashDirection`))
    ;[1 0.1569 0.1961] Control dash duration
    (set `self.dashDirection` _dashdirection)
    (set `self.dashing` true)
    (set `self.canHit` true)
    (`KismetSystemLibrary.Delay` (`self.dashTime`))
    (set `self.dashing` false)
    (set `self.canHit` false)))

(event `self.CapsuleComponent.OnComponentHit`
  (params (HitComponent :type "PrimitiveComponent Object Reference") (OtherActor :type "Actor Object Reference") (OtherComp :type "PrimitiveComponent Object Reference") (NormalImpulse :type "Vector Structure") (Hit :type "HitResult Structure (by ref)"))
  ;[1 0.1569 0.1961] Hit on Capsule Component
  (`|ExecutionSequence`
    (:`then_1`
      ;[0.3765 0.6863 1] Stop moving on collision
      (set `self.dashing` false)
      ;[0.3882 1 0.3333] Wait then disable can hit
      (`KismetSystemLibrary.Delay` 0.05)
      (set `self.canHit` false))))

(fn `GetDashDirection`
  (returns (dashDirection :type "Vector Structure"))
  (bind _playercontroller (`self.playerController`))
  (bind (_locationx _locationy) (`PlayerController.GetMousePosition` _playercontroller))
  (bind (_returnvalue_roll _returnvalue_pitch) (`KismetMathLibrary.BreakRotator` (`SceneComponent.K2_GetComponentRotation` (`self.Cone`))))
  (bind (_returnvalue_roll_2 _returnvalue_pitch_2 _returnvalue_yaw) (`KismetMathLibrary.BreakRotator` (`KismetMathLibrary.Conv_VectorToRotator` (`KismetMathLibrary.Vector_ToDegrees` (`KismetMathLibrary.Vector_ToRadians` (`KismetMathLibrary.MakeVector` 0.0))))))
  ;[1 1 1] Get direction vector (from player to click position)
  (bind _returnvalue (`self.GetMousePositionFromPlayer` (`PlayerController.ProjectWorldLocationToScreen` _playercontroller (`self.K2_GetActorLocation`) false) (`KismetMathLibrary.MakeVector2D` _locationx _locationy)))
  ;[1 1 1] Make player face click direction
  (`SceneComponent.K2_SetRelativeRotation` (`self.Cone`) (`KismetMathLibrary.MakeRotator` _returnvalue_yaw _returnvalue_pitch _returnvalue_roll_2) false false)
  (return (`KismetMathLibrary.Normal` (`KismetMathLibrary.Conv_Vector2DToVector` _returnvalue))))

(fn `UserConstructionScript`)